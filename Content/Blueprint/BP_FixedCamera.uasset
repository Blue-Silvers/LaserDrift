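; BP_FixedCamera is a camera Blueprint that follows the player character along the world Y axis only.
; On BeginPlay it caches player 0 as BP_Character and sets its rotation to the negated control rotation, printing an error if the cast fails.
; Each Tick moves its capsule to the character's Y while keeping its own X and Z, and copies the control rotation, without validating the cached reference.
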(event EventBeginPlay
  (bind _asbp_character (Utilities|Casting|CastToBP_Character (Game|GetPlayerCharacter 0))
    (:then
      (Variables|Default|SetAs%20BP%20Character _asbp_character)
      (Transformation|SetActorRotation (Class|KismetMathLibrary|NegateRotator (Pawn|GetControlRotation (Variables|Default|GetAs%20BP%20Character) :!class /Script/Engine.Pawn))))
    (:CastFailed
      (Development|PrintString "No player  !"))))

(event EventTick
  (params (DeltaSeconds :type Float%20%28single-precision%29))
  (bind _as_bp_character (Variables|Default|GetAs%20BP%20Character))
  (bind _capsulecomponent (Variables|Collision|GetCapsuleComponent))
  (bind _returnvalue (Transformation|GetWorldLocation _capsulecomponent))
  (Transformation|SetWorldLocationAndRotation (Variables|Collision|GetCapsuleComponent) (Math|Vector|MakeVector (.x _returnvalue) (.y (Transformation|GetWorldLocation (Variables|/Script/Engine.Actor|GetRootComponent _as_bp_character))) (.z _returnvalue)) (Pawn|GetControlRotation _as_bp_character :!class /Script/Engine.Pawn) false false))

(fn ConstructionScript)