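; Player character that constantly advances along its control rotation, with its camera attached to the level's BP_FixedCamera at BeginPlay.
; Move input tilts the mesh through a timeline, and dash teleports along controller up/right axes, stopping at the line-trace impact point.
; Held inputs speed up or slow global time, restoring it on release.
; Hitting a "Laser"-tagged actor reloads the level, and pause toggles a lazily created BP_PauseMenu.
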(event OnComponentHit(CapsuleComponent)
  (params (HitComponent :type Primitive%20Component%20Object%20Reference) (OtherActor :type Actor%20Object%20Reference) (OtherComp :type Primitive%20Component%20Object%20Reference) (NormalImpulse :type Vector :default "0, 0, 0") (Hit :type Hit%20Result%20Structure%20%28by%20ref%29))
  (if (Actor|ActorHasTag OtherActor "Laser")
    (bind _returnvalue (Game|GetCurrentLevelName true))
    (Game|OpenLevel(byName) (Utilities|String|StringToName _returnvalue))))

(event Input|EnhancedActionEvents|EnhancedInputActionIA_AccelerateTime
  (params (ActionValue :type Boolean) (ElapsedSeconds :type Float%20%28double-precision%29) (TriggeredSeconds :type Float%20%28double-precision%29) (InputAction :type Input%20Action%20Object%20Reference :default "/Game/Input/IA_AccelerateTime.IA_AccelerateTime"))
  ;[1 1 1] Change time dilatation
  ;;[0 0 0] Accelerate
  (:Started
    (Utilities|Time|SetGlobalTimeDilation (Variables|Default|GetAccelerateTime)))
  (:Canceled
    (Utilities|Time|SetGlobalTimeDilation 1.0 :!label _label))
  (:Completed
    (goto _label)))

(event Input|EnhancedActionEvents|EnhancedInputActionIA_Pause
  (params (ActionValue :type Boolean) (ElapsedSeconds :type Float%20%28double-precision%29) (TriggeredSeconds :type Float%20%28double-precision%29) (InputAction :type Input%20Action%20Object%20Reference :default "/Game/Input/IA_Pause.IA_Pause"))
  (bind _returnvalue (Game|GetPlayerController 0))
  (bind _returnvalue_2 (Game|GetPlayerController 0))
  ;[0.3854 0.3854 0.3854] Pause
  (:Started
    (Utilities|IsValid (Variables|Default|GetPauseRef)
      (:Is%20Valid
        _)
      (:Is%20Not%20Valid
        (bind _returnvalue_3 (UserInterface|CreateWidget "/Game/Menus/Viewport/BP_PauseMenu.BP_PauseMenu_C"))
        (Variables|Default|SetPauseRef _returnvalue_3)))
    (if (Game|IsGamePaused)
      (Widget|RemovefromParent (Variables|Default|GetPauseRef))
      (Game|SetGamePaused false)
      (Variables|/Script/Engine.PlayerController|SetbShowMouseCursor _returnvalue_2 false)
      (Input|SetInputModeGameOnly _returnvalue_2 false)
      (else
        (UserInterface|Viewport|AddtoViewport (Variables|Default|GetPauseRef) 0)
        (Game|SetGamePaused true)
        (Variables|/Script/Engine.PlayerController|SetbShowMouseCursor _returnvalue true)
        (Input|SetInputModeUIOnly _returnvalue 0 "DoNotLock" false)
        (Widget|SetKeyboardFocus (Variables|/Game/Menus/Viewport/BP_PauseMenu.BP_PauseMenu_C|GetResumeButton (Variables|Default|GetPauseRef)))))))

(event Input|EnhancedActionEvents|EnhancedInputActionIA_SlowTime
  (params (ActionValue :type Boolean) (ElapsedSeconds :type Float%20%28double-precision%29) (TriggeredSeconds :type Float%20%28double-precision%29) (InputAction :type Input%20Action%20Object%20Reference :default "/Game/Input/IA_SlowTime.IA_SlowTime"))
  ;[1 1 1] Change time dilatation
  ;;[0 0 0] Slowing
  (:Started
    (Utilities|Time|SetGlobalTimeDilation (Variables|Default|GetSlowingTime)))
  (:Canceled
    (Utilities|Time|SetGlobalTimeDilation 1.0 :!label _label))
  (:Completed
    (goto _label)))

(event Input|EnhancedActionEvents|EnhancedInputActionIA_Dash
  (params (ActionValue :type Boolean) (ElapsedSeconds :type Float%20%28double-precision%29) (TriggeredSeconds :type Float%20%28double-precision%29) (InputAction :type Input%20Action%20Object%20Reference :default "/Game/Input/IA_Dash.IA_Dash"))
  (bind _returnvalue (Transformation|GetActorLocation))
  (bind _returnvalue_2 (Pawn|GetController))
  (bind _x (Variables|Default|GetX))
  (bind _y (Variables|Default|GetY))
  (bind _teleportforce (Variables|Default|GetTeleportForce))
  (bind _returnvalue_3 (Transformation|GetActorUpVector _returnvalue_2))
  (bind _returnvalue_4 (Transformation|GetActorRightVector _returnvalue_2))
  (bind _returnvalue_5 (* _y _teleportforce))
  (bind _returnvalue_6 (* _x _teleportforce))
  (bind _returnvalue_7 (* _returnvalue_3 _returnvalue_6))
  (bind _returnvalue_8 (* _returnvalue_4 _returnvalue_5))
  (bind _returnvalue_9 (+ _returnvalue _returnvalue_7 _returnvalue_8))
  ;[0 0 0] Dash
  (:Started
    (Variables|Default|SetTeleportationPoint _returnvalue_9)
    (bind (_outhit _returnvalue_10) (Collision|LineTraceForObjects _returnvalue _returnvalue_9 (Utilities|Array|MakeArray "ObjectTypeQuery2" "ObjectTypeQuery1" "ObjectTypeQuery3") false 0 "ForDuration"))
    (if _returnvalue_10
      (Variables|Default|SetTeleportationPoint (.ImpactPoint (Collision|BreakHitResult _outhit))))
    (Transformation|Teleport (Variables|Default|GetTeleportationPoint) "0, 0, 0")))

(event Input|EnhancedActionEvents|EnhancedInputActionIA_Move
  (params (ActionValue :type Vector%202D%20Structure) (ElapsedSeconds :type Float%20%28double-precision%29) (TriggeredSeconds :type Float%20%28double-precision%29) (InputAction :type Input%20Action%20Object%20Reference :default "/Game/Input/IA_Move.IA_Move"))
  (bind _mesh (Variables|Character|GetMesh))
  (bind _returnvalue (Transformation|GetWorldRotation _mesh))
  ;[0 0 0] Rotate
  (:Triggered
    (bind _newtrack_0 (Timeline|SmoothRotate Play)
      (:Update
        (Transformation|SetWorldRotation _mesh (Math|Rotator|MakeRotator (.roll _returnvalue) (Math|Float|Lerp (.pitch _returnvalue) (* (.Y (Math|Vector2D|BreakVector2D ActionValue)) 1e+01) _newtrack_0) (.yaw _returnvalue)) false false))))
  (:Canceled
    (Timeline|SmoothRotate SetNewTime))
  (:Completed
    (Timeline|SmoothRotate SetNewTime)))

(event EventBeginPlay
  (bind _returnvalue (Actor|GetActorOfClass "/Game/Blueprint/BP_FixedCamera.BP_FixedCamera_C"))
  (Transformation|AttachComponentToComponent (Variables|Default|GetCamera) (Variables|/Game/Blueprint/BP_FixedCamera.BP_FixedCamera_C|GetArrow1 _returnvalue) "None" "KeepRelative" "KeepRelative" "KeepRelative" true))

(event EventTick
  (params (DeltaSeconds :type Float%20%28single-precision%29))
  (Pawn|Input|AddMovementInput (Math|Vector|GetForwardVector (Pawn|GetControlRotation :!class /Script/Engine.Pawn)) (Variables|Default|GetSpeed) false))

(fn ConstructionScript)