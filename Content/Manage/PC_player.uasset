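; PC_player is the player controller that caches the BP_Character pawn on BeginPlay, adds the IMC_Mapping input context and handles its input.
; IA_Move drives the character along its up and right vectors, with a test action for forward movement.
; Dash instantly offsets it along local Y.
; Both accelerate and slow-time inputs set the controller's own CustomTimeDilation to AccelerateTime, restoring normal speed when released or canceled.
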(event Input|EnhancedActionEvents|EnhancedInputActionIA_AccelerateTime
  (params (ActionValue :type Boolean) (ElapsedSeconds :type Float%20%28double-precision%29) (TriggeredSeconds :type Float%20%28double-precision%29) (InputAction :type Input%20Action%20Object%20Reference :default "/Game/Input/IA_AccelerateTime.IA_AccelerateTime"))
  ;[1 1 1] Change time dilatation
  ;;[0 0 0] Accelerate
  (:Started
    (Variables|Default|SetCustomTimeDilation (Variables|Default|GetAccelerateTime)))
  (:Canceled
    (Variables|Default|SetCustomTimeDilation 1.0 :!label _label))
  (:Completed
    (goto _label)))

(event Input|EnhancedActionEvents|EnhancedInputActionIA_Move
  (params (ActionValue :type Vector%202D%20Structure) (ElapsedSeconds :type Float%20%28double-precision%29) (TriggeredSeconds :type Float%20%28double-precision%29) (InputAction :type Input%20Action%20Object%20Reference :default "/Game/Input/IA_Move.IA_Move"))
  (bind (_x _y) (Math|Vector2D|BreakVector2D ActionValue))
  (bind _as_bp_character (Variables|Default|GetAs%20BP%20Character))
  ;[1 1 1] Movement
  (Pawn|Input|AddMovementInput _as_bp_character (Transformation|GetActorUpVector _as_bp_character) _x false)
  (Pawn|Input|AddMovementInput _as_bp_character (Transformation|GetActorRightVector _as_bp_character) _y false))

(event Input|EnhancedActionEvents|EnhancedInputActionIA_SlowTime
  (params (ActionValue :type Boolean) (ElapsedSeconds :type Float%20%28double-precision%29) (TriggeredSeconds :type Float%20%28double-precision%29) (InputAction :type Input%20Action%20Object%20Reference :default "/Game/Input/IA_SlowTime.IA_SlowTime"))
  ;[1 1 1] Change time dilatation
  ;;[0 0 0] Slowing
  (:Started
    (Variables|Default|SetCustomTimeDilation (Variables|Default|GetAccelerateTime)))
  (:Canceled
    (Variables|Default|SetCustomTimeDilation 1.0 :!label _label))
  (:Completed
    (goto _label)))

(event Input|EnhancedActionEvents|EnhancedInputActionIA_Dash
  (params (ActionValue :type Boolean) (ElapsedSeconds :type Float%20%28double-precision%29) (TriggeredSeconds :type Float%20%28double-precision%29) (InputAction :type Input%20Action%20Object%20Reference :default "/Game/Input/IA_Dash.IA_Dash"))
  (bind _as_bp_character (Variables|Default|GetAs%20BP%20Character))
  (:Started
    (Class|Actor|AddActorLocalTransform _as_bp_character (Math|Transform|MakeTransform (Math|Vector|MakeVector 0.0 8e+02 0.0) "0, 0, 0" (Transformation|GetActorScale3D _as_bp_character)) false false)))

(event Input|EnhancedActionEvents|EnhancedInputActionIA_ForwardTest
  (params (ActionValue :type Vector%202D%20Structure) (ElapsedSeconds :type Float%20%28double-precision%29) (TriggeredSeconds :type Float%20%28double-precision%29) (InputAction :type Input%20Action%20Object%20Reference :default "/Game/Input/IA_ForwardTest.IA_ForwardTest"))
  (bind _as_bp_character (Variables|Default|GetAs%20BP%20Character))
  ;[1 0 0] Test
  (Pawn|Input|AddMovementInput _as_bp_character (Transformation|GetActorForwardVector _as_bp_character) (.X (Math|Vector2D|BreakVector2D ActionValue)) false))

(event EventBeginPlay
  ;[1 1 1] Initiate cast and input
  (bind _asbp_character (Utilities|Casting|CastToBP_Character (Game|Player|GetPlayerPawn 0))
    (:then
      (Variables|Default|SetAs%20BP%20Character _asbp_character)
      (Input|AddMappingContext (PlayerController|LocalPlayerSubsystems|GetEnhancedInputLocalPlayerSubsystem self) "/Game/Input/IMC_Mapping.IMC_Mapping" 0 "(bIgnoreAllPressedKeysUntilRelease=True,bForceImmediately=False,bNotifyUserSettings=False)"))
    (:CastFailed
      (Development|PrintString "Character cast failed"))))

(fn ConstructionScript)