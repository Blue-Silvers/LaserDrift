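; BP_MovingLaser is a laser actor whose Cylinder component oscillates back and forth along its relative X axis.
; BeginPlay caches the cylinder's starting X only when TrueXFalseY is true; the false branch does nothing, so no Y motion exists.
; Every Tick sets relative X to that start plus a degree-based sine of time since creation, tuned by Speed and Distance, regardless of the flag.
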(event EventBeginPlay
  (if (Variables|Default|GetTrueX/FalseY)
    (Variables|Default|SetRelativeStartingLocationX (.x (.location (Transformation|GetRelativeTransform (Variables|Default|GetCylinder)))))))

(event EventTick
  (params (DeltaSeconds :type Float%20%28single-precision%29))
  (Transformation|SetRelativeLocation (Variables|Default|GetCylinder) (Math|Vector|MakeVector (+ (Variables|Default|GetRelativeStartingLocationX) (* (Math|Trig|Sin(Degrees) (* (Actor|GetGameTimeSinceCreation) (Variables|Default|GetSpeed))) (Variables|Default|GetDistance))) 0.0 0.0) false false))

(fn ConstructionScript
  (|CallParentFunction))